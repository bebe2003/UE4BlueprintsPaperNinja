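; PNPickupCoinActor is a coin pickup that spins on a timeline-driven yaw and is collected when a PNPlayerPawn overlaps its box trigger.
; A timer opens a Gate one second after BeginPlay, so earlier overlaps are ignored.
; On collection it destroys itself, adds one coin to the pawn, and spawns a particle effect and sound at its location.
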(event `self.ReceiveBeginPlay`
  (`KismetSystemLibrary.K2_SetTimer` null "EnablePickup" 1.0)
  (bind (_direction _coinyaw) (`Timeline|CoinRotationTimeline`)
    (:`Update`
      (`SceneComponent.K2_SetRelativeRotation` (`self.StaticMeshComponent`) (`KismetMathLibrary.MakeRotator` 0.0 0.0 _coinyaw) false false))))

(event `EnablePickup`
  (goto _label :!via `Open`))

(event `self.BoxTrigger.OnComponentBeginOverlap`
  (params (OverlappedComponent :type "PrimitiveComponent Object Reference") (OtherActor :type "Actor Object Reference") (OtherComp :type "PrimitiveComponent Object Reference") (OtherBodyIndex :type Integer) (bFromSweep :type Boolean) (SweepResult :type "HitResult Structure (by ref)"))
  (bind (_aspnplayer_pawn _bsuccess) (cast `/Game/BluePrints/PNPlayerPawn` OtherActor :!pure true))
  (`/Engine/EditorBlueprintResources/StandardMacros.Gate` true :!label _label
    (:`Exit`
      (if _bsuccess
        (`self.K2_DestroyActor`)
        (`/Game/BluePrints/PNPlayerPawn.AddCoin` _aspnplayer_pawn 1)
        (`GameplayStatics.SpawnEmitterAtLocation` "/Game/Particles/PS_Pickup_Coin.PS_Pickup_Coin" (`self.K2_GetActorLocation`))
        (`GameplayStatics.PlaySoundAtLocation` "/Game/Audio/Cue/obj_coin_get_Cue.obj_coin_get_Cue" (`self.K2_GetActorLocation`) (struct) 1.0 1.0 0.0 null null null)))))

(fn `UserConstructionScript`)