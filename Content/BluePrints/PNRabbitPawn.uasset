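; PNRabbitPawn is a hostile rabbit character that damages the player by contact and hurts whatever blocks it while sprinting.
; Pawn sensing stores the seen player and sets the sprint flag, which enables a per-tick forward trace from the Spine socket to apply damage.
; Capsule hits also damage the player.
; Functions for sprint speed switching and trace-based player detection are exposed but not called within this Blueprint.
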(event `self.ReceiveBeginPlay`
  (set `CharacterMovementComponent.MaxWalkSpeed` (`self.WalkGoundSpeed`) (`self.CharacterMovement`)))

(event `self.ReceiveTick`
  (params (DeltaSeconds :type "Float (single-precision)"))
  (bind _returnvalue (`SceneComponent.GetSocketLocation` (`self.Mesh`) "Spine"))
  (if (`self.isSprint`)
    (bind _outhit (`KismetSystemLibrary.LineTraceSingle` _returnvalue (+ _returnvalue (* (`self.GetActorForwardVector`) (`self.TargetSight`))) "TraceTypeQuery1"))
    (bind (_bblockinghit _binitialoverlap _time _distance _location _impactpoint _normal _impactnormal _physmat _hitactor) (`GameplayStatics.BreakHitResult` _outhit))
    (if _bblockinghit
      (`GameplayStatics.ApplyDamage` _hitactor 100.0))))

(event `self.CapsuleComponent.OnComponentHit`
  (params (HitComponent :type "PrimitiveComponent Object Reference") (OtherActor :type "Actor Object Reference") (OtherComp :type "PrimitiveComponent Object Reference") (NormalImpulse :type "Vector Structure") (Hit :type "HitResult Structure (by ref)"))
  (`GameplayStatics.ApplyDamage` (cast `/Game/BluePrints/PNPlayerPawn` OtherActor :!pure true) 100.0))

(event `self.PawnSensing.OnSeePawn`
  (params (Pawn :type "Pawn Object Reference"))
  (bind (_aspnplayer_pawn _bsuccess) (cast `/Game/BluePrints/PNPlayerPawn` Pawn :!pure true))
  (set `self.SeenActor` _aspnplayer_pawn)
  (set `self.isSprint` _bsuccess))

(fn `BeginSprint`
  (set `CharacterMovementComponent.MaxWalkSpeed` (`self.SprintGroundSpeed`) (`self.CharacterMovement`))
  (set `self.isSprint` true))

(fn `CanSeePlayerPawn`
  (returns (isPlayer :type Boolean) (SeenActor :type "Actor Object Reference"))
  (bind _returnvalue (`self.K2_GetActorLocation`))
  (bind _outhit (`KismetSystemLibrary.LineTraceSingle` :`Start` _returnvalue :`End` (+ _returnvalue (* (`self.GetActorForwardVector`) (`self.SightLength`))) :`TraceChannel` "TraceTypeQuery3" :`DrawDebugType` "ForOneFrame"))
  (bind (_aspnplayer_pawn _bsuccess) (cast `/Game/BluePrints/PNPlayerPawn` (`.HitActor` (`GameplayStatics.BreakHitResult` _outhit)) :!pure true))
  (return _bsuccess _aspnplayer_pawn))

(fn `EndSprint`
  (set `CharacterMovementComponent.MaxWalkSpeed` (`self.WalkGoundSpeed`) (`self.CharacterMovement`))
  (set `self.isSprint` false)
  (set `self.SeenActor` (`self.EmtyActor`)))

(fn `UserConstructionScript`)